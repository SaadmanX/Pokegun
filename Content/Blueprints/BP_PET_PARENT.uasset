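; Parent Blueprint for pets that accompany the top-down player and battle other pets using HP, mana and level.
; Tick sets MovingSprite from 2D distance to the player and refreshes the health bar widget, which is hidden on possession.
; Attack, defend, heal and slash functions roll random outcomes, adjust stats and set animation states through Blackboards.
; The special move paralyzes or poisons the enemy, with choice and odds based on level.
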(event `self.ReceivePossessed`
  (params (NewController :type "Controller Object Reference"))
  (bind _returnvalue (`GameplayStatics.GetActorOfClass` "/Game/Blueprints/PLAYER_BLUEPRINTS/BP_TopDownChar.BP_TopDownChar_C"))
  (set `self.player` _returnvalue)
  (set `self.moving_sprite` false)
  (`SceneComponent.SetVisibility` (`self.HealthBar`) false false))

(event `self.ReceiveTick`
  (params (DeltaSeconds :type "Float (single-precision)"))
  (`/Engine/EditorBlueprintResources/StandardMacros.CompareFloat` (`KismetMathLibrary.Distance2D` (`KismetMathLibrary.Conv_VectorToVector2D` (`self.K2_GetActorLocation` (`self.player`))) (`KismetMathLibrary.Conv_VectorToVector2D` (`self.K2_GetActorLocation`))) 200.0
    (:`>`
      (set `self.moving_sprite` true))
    (:`==`
      (set `self.moving_sprite` false :!label _label))
    (:`<`
      (goto _label)))
  ; Health + Mana Bar + Level
  (bind _aswb_health_bar (cast `/Game/Assets/HealthBar/WB_HealthBar` (`WidgetComponent.GetWidget` (`self.HealthBar`))))
  (`ProgressBar.SetPercent` (`/Game/Assets/HealthBar/WB_HealthBar.HealthBar` _aswb_health_bar) (/ (`self.hp`) (`self.maxHp`)))
  (`ProgressBar.SetPercent` (`/Game/Assets/HealthBar/WB_HealthBar.ManaBar` _aswb_health_bar) (/ (`self.mana`) (`self.maxMana`)))
  (`TextBlock.SetText` (`/Game/Assets/HealthBar/WB_HealthBar.Level` _aswb_health_bar) (`KismetTextLibrary.Conv_IntToText` (`self.level`))))

(fn `Handle Attack`
  (params (`Enemy Pet` :type "/Game/Blueprints/BP_PET_PARENT Object Reference"))
  (locals (EnemyPet :type "/Game/Blueprints/BP_PET_PARENT Object Reference"))
  (bind _enemypet (`local.EnemyPet`))
  (bind _enemypet_2 (`local.EnemyPet`))
  (bind _output_get (set `local.EnemyPet` `Enemy Pet`))
  (`BlackboardComponent.SetValueAsInt` (`AIBlueprintHelperLibrary.GetBlackboard` self) "animationstate" 2)
  (`BlackboardComponent.SetValueAsInt` (`AIBlueprintHelperLibrary.GetBlackboard` _output_get) "animationstate" 5)
  (if (> (`KismetMathLibrary.RandomFloat`) 0.1)
    (bind _output_get_2 (set `/Game/Blueprints/BP_PET_PARENT.hp` (- (`/Game/Blueprints/BP_PET_PARENT.hp` (`local.EnemyPet`)) (`self.atk`)) _enemypet))
    (if (`/Game/Blueprints/BP_PET_PARENT.defSuccess` (`local.EnemyPet`))
      (set `/Game/Blueprints/BP_PET_PARENT.hp` (+ _output_get_2 (`/Game/Blueprints/BP_PET_PARENT.def` _enemypet)) _enemypet_2)
      (set `/Game/Blueprints/BP_PET_PARENT.defSuccess` false _enemypet_2)
      (if (< (`self.mana`) (`self.maxMana`))
        (bind _output_get_3 (set `self.mana` (+ (`self.mana`) 1)))
        (if (> _output_get_3 (`self.maxMana`))
          (set `self.mana` (`self.maxMana`)))))
    (else
      (`KismetSystemLibrary.PrintString` "Bad luck, you missed"))))

(fn `Handle Defend`
  (`BlackboardComponent.SetValueAsInt` (`AIBlueprintHelperLibrary.GetBlackboard` null) "animationstate" 3)
  (if (> (`KismetMathLibrary.RandomFloat`) 0.4)
    (set `self.defSuccess` false)
    (if (< (`self.mana`) (`self.maxMana`))
      (bind _output_get (set `self.mana` (+ (`self.mana`) 1)))
      (if (> _output_get (`self.maxMana`))
        (set `self.mana` (`self.maxMana`))))))

(fn `Handle Healing`
  (bind _maxhp (`self.maxHp`))
  (bind _maxhp_2 (`self.maxHp`))
  (bind _returnvalue (* (`self.hp`) 1.2))
  (bind _returnvalue_2 (* (`self.hp`) 1.1))
  (`BlackboardComponent.SetValueAsInt` (`AIBlueprintHelperLibrary.GetBlackboard` null) "animationstate" 4)
  (if (>= (`self.mana`) 3)
    (if (not (>= (`self.hp`) (`self.maxHp`)))
      (if (>= (`KismetMathLibrary.RandomFloat`) 0.8)
        (if (> _returnvalue _maxhp_2)
          (set `self.hp` _maxhp_2)
          (else
            (set `self.hp` _returnvalue)))
        (elif (> _returnvalue_2 _maxhp)
          (set `self.hp` _maxhp)
          (else
            (set `self.hp` _returnvalue_2))))
      (set `self.mana` (- (`self.mana`) 3))
      (if (< (`self.mana`) (`self.maxMana`))
        (bind _output_get (set `self.mana` (+ (`self.mana`) 1)))
        (if (> _output_get (`self.maxMana`))
          (set `self.mana` (`self.maxMana`)))))))

(fn `Handle Slash`
  (params (`Enemy Pet` :type "/Game/Blueprints/BP_PET_PARENT Object Reference"))
  (locals (EnemyPet :type "/Game/Blueprints/BP_PET_PARENT Object Reference"))
  (bind _output_get (set `local.EnemyPet` `Enemy Pet`))
  (`BlackboardComponent.SetValueAsInt` (`AIBlueprintHelperLibrary.GetBlackboard` self) "animationstate" 2)
  (`BlackboardComponent.SetValueAsInt` (`AIBlueprintHelperLibrary.GetBlackboard` _output_get) "animationstate" 6)
  (if (and (> (`KismetMathLibrary.RandomFloat`) 0.05) (>= (`self.mana`) (`self.slashMana`)))
    (set `self.mana` (- (`self.mana`) (`self.slashMana`)))
    (set `/Game/Blueprints/BP_PET_PARENT.hp` (- (`/Game/Blueprints/BP_PET_PARENT.hp` (`local.EnemyPet`)) (* (`self.atk`) 2)) (`local.EnemyPet`))
    (if (< (`self.mana`) (`self.maxMana`))
      (bind _output_get_2 (set `self.mana` (+ (`self.mana`) 1)))
      (if (> _output_get_2 (`self.maxMana`))
        (set `self.mana` (`self.maxMana`))))))

(fn `Make Special Move`
  (params (Enemy :type "/Game/Blueprints/BP_PET_PARENT Object Reference"))
  (bind _level (`self.level`))
  (bind _enemy (`local.Enemy`))
  (if (<= _level 7)
    (`self.Paralyze Enemy` _enemy :!label _label)
    (else
      (if (<= _level 9)
        _
        (elif (> (`KismetMathLibrary.RandomFloat`) 0.5)
          (goto _label)
          (else
            _)))
      (`self.Poison Enemy` _enemy))))

(fn `Paralyze Enemy`
  (params (Enemy :type "/Game/Blueprints/BP_PET_PARENT Object Reference"))
  (if (>= (* 0.12 (`self.level`)) (`KismetMathLibrary.RandomFloat`))
    (set `/Game/Blueprints/BP_PET_PARENT.isParalyzed` true (`local.Enemy`))))

(fn `Poison Enemy`
  (params (Enemy :type "/Game/Blueprints/BP_PET_PARENT Object Reference"))
  (bind _enemy (`local.Enemy`))
  (if (>= (* 0.1 (`self.level`)) (`KismetMathLibrary.RandomFloat`))
    (set `/Game/Blueprints/BP_PET_PARENT.poisonedCounter` (mod (`/Game/Blueprints/BP_PET_PARENT.level` _enemy) 7) _enemy)))

(fn `UserConstructionScript`)