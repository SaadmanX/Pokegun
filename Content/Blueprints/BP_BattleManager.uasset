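; BP_BattleManager runs a pet battle between PlayerPet and EnemyPet through a BP_BattleMenu widget.
; BeginPlay creates and binds the menu and spawns an owl pet actor without storing it.
; Attack, slash, heal and defend selections call PlayerPet handlers, then end the turn.
; Tick hides the menu for one frame, restores the player turn without an enemy action, and opens MainGame once either pet's HP runs out.
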(event `OnBattleActionSelected`
  (params (type :type String))
  ; Binding Battle Action Selection
  (if (`KismetStringLibrary.EqualEqual_StrStr` type "attack")
    (`self.OnAttackSelected`)
    (set `self.isPlayerTurn` false :!label _label)
    (`KismetSystemLibrary.PrintString` "Player health")
    (`KismetSystemLibrary.PrintString` (`KismetStringLibrary.Conv_DoubleToString` (`/Game/Blueprints/BP_Pet.hp` (`self.playerPet`))))
    (`KismetSystemLibrary.PrintString` "Boss Health: ")
    (`KismetSystemLibrary.PrintString` (`KismetStringLibrary.Conv_DoubleToString` (`/Game/Blueprints/BP_Pet.hp` (`self.enemyPet`))))
    (elif (`KismetStringLibrary.EqualEqual_StrStr` type "defend")
      (`self.OnDefendSelected`)
      (goto _label)
      (elif (`KismetStringLibrary.EqualEqual_StrStr` type "heal")
        (`self.OnHealSelected`)
        (goto _label)
        (elif (`KismetStringLibrary.EqualEqual_StrStr` type "slash")
          (`self.OnSlashSelected`)
          (goto _label))))))

(event `self.ReceiveBeginPlay`
  ; Battle Menu Initialization
  (bind _returnvalue (`|CreateWidget` "/Game/Blueprints/BP_BattleMenu.BP_BattleMenu_C"))
  (`UserWidget.AddToViewport` _returnvalue 0)
  (bind _output_get (set `self.BattleMenu` _returnvalue))
  (add `/Game/Blueprints/BP_BattleMenu.ActionSelected` _output_get (delegate `OnBattleActionSelected`))
  (`|SpawnActorFromClass` "/Game/Blueprints/PET_BLUEPRINTS/BP_PET_OWL_CHAR.BP_PET_OWL_CHAR_C" (`KismetMathLibrary.MakeTransform` (100.0 0.0 100.0)) "Undefined" "MultiplyWithRoot" null null))

(event `self.ReceiveTick`
  (params (DeltaSeconds :type "Float (single-precision)"))
  ; Battle Loop Logic
  (if (and (> (`/Game/Blueprints/BP_Pet.hp` (`self.playerPet`)) 0) (> (`/Game/Blueprints/BP_Pet.hp` (`self.enemyPet`)) 0))
    ; Turn-Based Logic
    (if (`self.isPlayerTurn`)
      (`Widget.SetVisibility` (`self.BattleMenu`) "Visible")
      (else
        (`Widget.SetVisibility` (`self.BattleMenu`) "Hidden")
        (set `self.isPlayerTurn` true)))
    (else
      (`KismetSystemLibrary.PrintString` "End Game")
      (`GameplayStatics.OpenLevel` "MainGame"))))

(event `OnAttackSelected`
  ; Handle Attack
  (`/Game/Blueprints/BP_Pet.Handle Attack` (`self.playerPet`) (`self.enemyPet`)))

(event `OnSlashSelected`
  ; Handle Slash
  (`/Game/Blueprints/BP_Pet.Handle Slash` (`self.playerPet`) (`self.enemyPet`)))

(event `OnHealSelected`
  ; Handle Healing
  (`/Game/Blueprints/BP_Pet.Handle Healing` (`self.playerPet`)))

(event `OnDefendSelected`
  ; Handle Defend
  (`/Game/Blueprints/BP_Pet.Handle Defend` (`self.playerPet`)))

(event `TriggerPetAction`)

(fn `UserConstructionScript`)