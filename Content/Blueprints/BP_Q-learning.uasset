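; Q-learning agent that picks and performs turn-based combat actions: attack, slash, heal or defend, apparently for the enemy.
; Epsilon-greedy selection reads a flat Q-table indexed by state and action, limiting random picks to attack or defend when mana is low.
; Performing an action predicts the next of eight states, which encode own health, mana and opponent health as bits.
; Health changes become the reward that updates the Q-table before the state advances.
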(fn `Get Q`
  (params (State :type Integer) (Action :type Integer))
  (returns (QValue :type "Float (double-precision)"))
  (return (`|GetArrayItem` (`self.QTable`) (+ (* State 4) Action))))

(fn `Perform Action + Observe`
  (params (state :type Integer) (Action :type Integer) (enemy :type "/Game/Blueprints/BP_PET_PARENT Object Reference") (player :type "/Game/Blueprints/BP_PET_PARENT Object Reference"))
  (locals (cState :type Integer) (cAction :type Integer))
  (bind _player (`local.player`))
  (bind _cstate (`local.cState`))
  (bind _cstate_2 (`local.cState`))
  (bind _cstate_3 (`local.cState`))
  (bind _returnvalue (or (== (`local.cState`) 2) (== (`local.cState`) 3) (== (`local.cState`) 6) (== (`local.cState`) 7)))
  ; Perform Action
  (set `local.cState` state)
  (set `self.lastEnemyHealth` (`/Game/Blueprints/BP_PET_PARENT.hp` enemy))
  (set `self.lastPlayerHealth` (`/Game/Blueprints/BP_PET_PARENT.hp` player))
  (if (== Action 0)
    (`/Game/Blueprints/BP_PET_PARENT.Handle Attack` (`local.player`) (`local.enemy`))
    (`KismetSystemLibrary.PrintString` "Enemy Attacked!")
    ; Observe next State
    (if (and (or (== (`local.cState`) 1) (== (`local.cState`) 3) (== (`local.cState`) 5) (== (`local.cState`) 7)) (<= (`/Game/Blueprints/BP_PET_PARENT.hp` (`local.enemy`)) (* (`/Game/Blueprints/BP_PET_PARENT.maxHp` (`local.enemy`)) 0.5))) :!label _label
      (set `self.NextState` (- _cstate 1))
      (else
        (set `self.NextState` _cstate)))
    (if (and (not _returnvalue) (<= (`/Game/Blueprints/BP_PET_PARENT.slashMana` (`local.player`)) (`/Game/Blueprints/BP_PET_PARENT.mana` (`local.player`))))
      (set `self.NextState` (+ (`local.cState`) 2)))
    (elif (== Action 1)
      (`/Game/Blueprints/BP_PET_PARENT.Handle Slash` (`local.player`) (`local.enemy`))
      (`KismetSystemLibrary.PrintString` "Enemy Slash")
      (if (and _returnvalue (< (`/Game/Blueprints/BP_PET_PARENT.mana` (`local.player`)) (`/Game/Blueprints/BP_PET_PARENT.slashMana` (`local.player`))))
        (set `local.cState` (- _cstate_2 2))
        (goto _label)
        (else
          (set `local.cState` _cstate_2)))
      (elif (== Action 2)
        (`/Game/Blueprints/BP_PET_PARENT.Handle Healing` (`local.player`))
        (`KismetSystemLibrary.PrintString` "Enemy heal")
        (if (and (<= (`local.cState`) 3) (>= (`/Game/Blueprints/BP_PET_PARENT.hp` _player) (* (`/Game/Blueprints/BP_PET_PARENT.maxHp` _player) 0.5)))
          (set `self.NextState` (+ _cstate_3 4))
          (else
            (set `self.NextState` _cstate_3)))
        (else
          (`/Game/Blueprints/BP_PET_PARENT.Handle Defend` (`local.player`))
          (`KismetSystemLibrary.PrintString` "Enemy defends")
          (set `self.NextState` (`local.cState`)))))))

(fn `Receive Reward`
  (params (`Player Current Health` :type "Float (double-precision)") (`Enemy Current Health` :type "Float (double-precision)"))
  (returns (Rewards :type "Float (double-precision)"))
  (if (< `Enemy Current Health` (`self.lastEnemyHealth`))
    (return (- (`self.lastEnemyHealth`) (`local.Enemy Current Health`)))
    (elif (> (`local.Player Current Health`) (`self.lastPlayerHealth`))
      (return (- (`local.Player Current Health`) (`self.lastPlayerHealth`) (- (`local.Enemy Current Health`) (`self.lastEnemyHealth`))))
      (else
        (return (- (`local.Player Current Health`) (`self.lastPlayerHealth`) (- (`local.Enemy Current Health`) (`self.lastEnemyHealth`))))))))

(fn `Select Action`
  (params (State :type Integer))
  (returns (`Action Index` :type Integer))
  (locals (CurrentState :type Integer :default 7) (maxQ :type "Float (double-precision)" :default -10000.0) (epsilon :type "Float (double-precision)" :default 0.2) (returnedAction :type Integer) (index :type Integer))
  (bind _returnedaction (`local.returnedAction`))
  (if (<= (`KismetMathLibrary.RandomFloat`) (`local.epsilon`))
    (if (or (== (`local.CurrentState`) 2) (== (`local.CurrentState`) 3) (== (`local.CurrentState`) 6) (== (`local.CurrentState`) 7))
      (return (`KismetMathLibrary.RandomInteger` 4))
      (elif (< (`KismetMathLibrary.RandomInteger` 4) 2)
        (return 0)
        (else
          (return 3))))
    (else
      (for _index (range 4)
        (bind _output_get (set `local.index` _index))
        (bind _qvalue (`self.Get Q` (`local.State`) _output_get))
        (if (> _qvalue (`local.maxQ`))
          (set `local.maxQ` _qvalue)
          (set `local.returnedAction` (`local.index`))))
      (`KismetSystemLibrary.PrintString` (`KismetStringLibrary.Concat_StrStr` "Choosing Action" (`KismetStringLibrary.Conv_IntToString` _returnedaction)))
      (return _returnedaction))))

(fn `Set Q`
  (params (State :type Integer) (Value :type "Float (double-precision)") (Action :type Integer))
  (`KismetArrayLibrary.Array_Set` (`self.QTable`) (+ (* State 4) Action) Value))

(fn `Update QTable`
  (params (Action :type Integer) (Rewards :type "Float (double-precision)"))
  (locals (alpha :type "Float (double-precision)" :default 1.0) (gamma :type "Float (double-precision)" :default 0.7) (maxNextState :type "Float (double-precision)") (maxQ :type "Float (double-precision)" :default -1000.0) (curQ :type "Float (double-precision)"))
  (bind _qvalue (`self.Get Q` (`self.State`) Action))
  (bind _output_get (set `local.curQ` _qvalue))
  (for _index (range 4)
    (bind _qvalue_2 (`self.Get Q` (`self.NextState`) _index))
    (if (> _qvalue_2 (`local.maxQ`))
      (set `local.maxQ` _qvalue_2)))
  (`self.Set Q` (`self.State`) (+ _output_get (* (`local.alpha`) (+ (`local.Rewards`) (* (- (`local.maxQ`) (`local.curQ`)) (`local.gamma`))))) (`local.Action`)))

(fn `Update State`
  (returns (ReturnedState :type Integer))
  (locals (cState :type Integer) (cAction :type Integer))
  ; Transit to next state
  (bind _output_get (set `self.State` (`self.NextState`)))
  (return _output_get))

(fn `UserConstructionScript`)