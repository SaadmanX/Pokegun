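; Parent pet Blueprint for turn-based-style battles, holding stats and combat actions for friendly and enemy pets.
; Attack, defend, heal, slash and level-gated paralyze or poison use random rolls, then report through BattleLog and sound.
; AI Blackboard keys select animations and identify the friendly side.
; Tick refreshes the health bar widget, flags sprite movement by player distance and forces velocity to orient pets per level.
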(event `self.ReceiveBeginPlay`
  (bind _returnvalue (`GameplayStatics.GetActorOfClass` "/Game/Blueprints/PLAYER_BLUEPRINTS/BP_TopDownChar.BP_TopDownChar_C"))
  (set `self.player` _returnvalue)
  (set `self.moving_sprite` false)
  (`SceneComponent.SetVisibility` (`self.HealthBar`) false false)
  (set `self.isInitialized` true))

(event `self.ReceiveTick`
  (params (DeltaSeconds :type "Float (single-precision)"))
  (bind _charactermovement (`self.CharacterMovement`))
  (if (`self.isInitialized`)
    (`/Engine/EditorBlueprintResources/StandardMacros.CompareFloat` (`KismetMathLibrary.Distance2D` (`KismetMathLibrary.Conv_VectorToVector2D` (`self.K2_GetActorLocation` (`self.player`))) (`KismetMathLibrary.Conv_VectorToVector2D` (`self.K2_GetActorLocation`))) 200.0
      (:`>`
        (set `self.moving_sprite` true))
      (:`==`
        (set `self.moving_sprite` false :!label _label))
      (:`<`
        (goto _label)))
    ; Status Bar Values
    (bind _aswb_health_bar (cast `/Game/Assets/HealthBar/WB_HealthBar` (`WidgetComponent.GetWidget` (`self.HealthBar`))))
    (`ProgressBar.SetPercent` (`/Game/Assets/HealthBar/WB_HealthBar.HealthBar` _aswb_health_bar) (/ (`self.hp`) (`self.maxHp`)))
    (`ProgressBar.SetPercent` (`/Game/Assets/HealthBar/WB_HealthBar.ManaBar` _aswb_health_bar) (/ (`self.mana`) (`self.maxMana`)))
    (`TextBlock.SetText` (`/Game/Assets/HealthBar/WB_HealthBar.Level` _aswb_health_bar) (`KismetTextLibrary.Conv_IntToText` (`self.level`)))
    (if (> (`self.poisonedCounter`) 0)
      (bind _poison (`/Game/Assets/HealthBar/WB_HealthBar.Poison` _aswb_health_bar))
      (`Widget.SetVisibility` _poison "Visible")
      (else
        (`Widget.SetVisibility` _poison "Hidden")))
    (if (`self.isParalyzed`)
      (bind _paralyzed (`/Game/Assets/HealthBar/WB_HealthBar.Paralyzed` _aswb_health_bar))
      (`Widget.SetVisibility` _paralyzed "Visible")
      (else
        (`Widget.SetVisibility` _paralyzed "Hidden")))
    (`TextBlock.SetText` (`/Game/Assets/HealthBar/WB_HealthBar.HealthNumber` _aswb_health_bar) (`KismetTextLibrary.Conv_DoubleToText` (`self.hp`) "HalfToEven" false true 1 324 1 1))
    (`TextBlock.SetText` (`/Game/Assets/HealthBar/WB_HealthBar.ManaNumber` _aswb_health_bar) (`KismetTextLibrary.Conv_IntToText` (`self.mana`)))
    ; Friendly Pet Orientation for Battle
    (bind _returnvalue (`GameplayStatics.GetCurrentLevelName` true))
    (if (and (`BlackboardComponent.GetValueAsBool` (`AIBlueprintHelperLibrary.GetBlackboard` null) "isFighting") (`BlackboardComponent.GetValueAsBool` (`AIBlueprintHelperLibrary.GetBlackboard` null) "isFriendly"))
      (bind _returnvalue_2 (`KismetStringLibrary.EqualEqual_StrStr` _returnvalue "BossLevel"))
      (if _returnvalue_2
        (set `MovementComponent.Velocity` (0.0 -10.0 0.0) _charactermovement)
        (else
          (set `MovementComponent.Velocity` (-10.0 0.0 0.0) _charactermovement)))
      (elif _returnvalue_2
        (set `MovementComponent.Velocity` (0.0 -10.0 0.0) _charactermovement)))))

(fn `Handle Attack`
  (params (`Enemy Pet` :type "/Game/Blueprints/PET_BLUEPRINTS/BP_PET_PARENT Object Reference"))
  (locals (EnemyPet :type "/Game/Blueprints/PET_BLUEPRINTS/BP_PET_PARENT Object Reference"))
  (bind _battlelog (`self.battleLog`))
  (bind _enemypet (`local.EnemyPet`))
  (bind _enemypet_2 (`local.EnemyPet`))
  (bind _battlelog_2 (`self.battleLog`))
  (bind _returnvalue (`AIBlueprintHelperLibrary.GetBlackboard` self))
  (bind _output_get (set `local.EnemyPet` `Enemy Pet`))
  (`BlackboardComponent.SetValueAsInt` _returnvalue "animationstate" 2)
  (`BlackboardComponent.SetValueAsBool` _returnvalue "isAnimating" true)
  (bind _returnvalue_2 (`AIBlueprintHelperLibrary.GetBlackboard` _output_get))
  (`BlackboardComponent.SetValueAsInt` _returnvalue_2 "animationstate" 5)
  (`BlackboardComponent.SetValueAsBool` _returnvalue_2 "isAnimating" true)
  (if (> (`KismetMathLibrary.RandomFloat`) 0.1)
    (bind _output_get_2 (set `/Game/Blueprints/PET_BLUEPRINTS/BP_PET_PARENT.hp` (- (`/Game/Blueprints/PET_BLUEPRINTS/BP_PET_PARENT.hp` (`local.EnemyPet`)) (`self.atk`)) _enemypet))
    (if (`/Game/Blueprints/PET_BLUEPRINTS/BP_PET_PARENT.defSuccess` (`local.EnemyPet`))
      (set `/Game/Blueprints/PET_BLUEPRINTS/BP_PET_PARENT.hp` (+ _output_get_2 (`/Game/Blueprints/PET_BLUEPRINTS/BP_PET_PARENT.def` _enemypet)) _enemypet_2)
      (set `/Game/Blueprints/PET_BLUEPRINTS/BP_PET_PARENT.defSuccess` false _enemypet_2))
    (if (`BlackboardComponent.GetValueAsBool` (`AIBlueprintHelperLibrary.GetBlackboard` null) "isFriendly")
      (`/Game/Assets/BattleAssets/BP_BattleLog.AddLogEntry` _battlelog_2 "You attacked the enemy!")
      (else
        (`/Game/Assets/BattleAssets/BP_BattleLog.AddLogEntry` _battlelog_2 "Enemy attacked you!")))
    (`GameplayStatics.PlaySound2D` "/Game/Assets/Sounds/SFX/Hit.Hit" 1.0 1.0 0.0 null null)
    (else
      (if (`BlackboardComponent.GetValueAsBool` (`AIBlueprintHelperLibrary.GetBlackboard` null) "isFriendly")
        (`/Game/Assets/BattleAssets/BP_BattleLog.AddLogEntry` _battlelog "Your attack missed!")
        (else
          (`/Game/Assets/BattleAssets/BP_BattleLog.AddLogEntry` _battlelog "Enemy attack missed!")))
      (`GameplayStatics.PlaySound2D` "/Game/Assets/Sounds/SFX/Fail.Fail" 1.0 1.0 0.0 null null))))

(fn `Handle Defend`
  (bind _returnvalue (`AIBlueprintHelperLibrary.GetBlackboard` null))
  (bind _battlelog (`self.battleLog`))
  (bind _battlelog_2 (`self.battleLog`))
  (`BlackboardComponent.SetValueAsInt` _returnvalue "animationstate" 3)
  (`BlackboardComponent.SetValueAsBool` _returnvalue "isAnimating" true)
  (if (> (`KismetMathLibrary.RandomFloat`) 0.4)
    (set `self.defSuccess` true)
    (if (`BlackboardComponent.GetValueAsBool` (`AIBlueprintHelperLibrary.GetBlackboard` null) "isFriendly")
      (`/Game/Assets/BattleAssets/BP_BattleLog.AddLogEntry` _battlelog_2 "Your defend succeeded!")
      (else
        (`/Game/Assets/BattleAssets/BP_BattleLog.AddLogEntry` _battlelog_2 "Enemy defend succeeded!")))
    (`GameplayStatics.PlaySound2D` "/Game/Assets/Sounds/SFX/PowerUp1.PowerUp1" 1.0 1.0 0.0 null null)
    (else
      (if (`BlackboardComponent.GetValueAsBool` (`AIBlueprintHelperLibrary.GetBlackboard` null) "isFriendly")
        (`/Game/Assets/BattleAssets/BP_BattleLog.AddLogEntry` _battlelog "Your defend failed!")
        (else
          (`/Game/Assets/BattleAssets/BP_BattleLog.AddLogEntry` _battlelog "Enemy defend failed!")))
      (`GameplayStatics.PlaySound2D` "/Game/Assets/Sounds/SFX/Fail.Fail" 1.0 1.0 0.0 null null))))

(fn `Handle Healing`
  (bind _returnvalue (`AIBlueprintHelperLibrary.GetBlackboard` null))
  (bind _battlelog (`self.battleLog`))
  (bind _maxhp (`self.maxHp`))
  (bind _battlelog_2 (`self.battleLog`))
  (bind _maxhp_2 (`self.maxHp`))
  (bind _poisonedcounter (`self.poisonedCounter`))
  (bind _returnvalue_2 (* (`self.hp`) 1.2))
  (bind _returnvalue_3 (* (`self.hp`) 1.1))
  (`BlackboardComponent.SetValueAsInt` _returnvalue "animationstate" 4)
  (`BlackboardComponent.SetValueAsBool` _returnvalue "isAnimating" true)
  (if (>= (`self.mana`) 3)
    (if (>= (`self.hp`) (`self.maxHp`))
      (if (`BlackboardComponent.GetValueAsBool` (`AIBlueprintHelperLibrary.GetBlackboard` null) "isFriendly") :!label _label
        (`/Game/Assets/BattleAssets/BP_BattleLog.AddLogEntry` _battlelog "Your heal failed!")
        (else
          (`/Game/Assets/BattleAssets/BP_BattleLog.AddLogEntry` _battlelog "Enemy heal failed!")))
      (`GameplayStatics.PlaySound2D` "/Game/Assets/Sounds/SFX/Fail.Fail" 1.0 1.0 0.0 null null)
      (else
        (if (>= (`KismetMathLibrary.RandomFloat`) 0.8)
          (if (> _returnvalue_2 _maxhp_2)
            (set `self.hp` _maxhp_2)
            (else
              (set `self.hp` _returnvalue_2)))
          (elif (> _returnvalue_3 _maxhp)
            (set `self.hp` _maxhp)
            (else
              (set `self.hp` _returnvalue_3))))
        (set `self.mana` (- (`self.mana`) 3))
        (if (> _poisonedcounter 0)
          (set `self.poisonedCounter` (- _poisonedcounter 1)))
        (if (`BlackboardComponent.GetValueAsBool` (`AIBlueprintHelperLibrary.GetBlackboard` null) "isFriendly")
          (`/Game/Assets/BattleAssets/BP_BattleLog.AddLogEntry` _battlelog_2 "You healed!")
          (else
            (`/Game/Assets/BattleAssets/BP_BattleLog.AddLogEntry` _battlelog_2 "Enemy healed!")))
        (`GameplayStatics.PlaySound2D` "/Game/Assets/Sounds/SFX/Magic1.Magic1" 1.0 1.0 0.0 null null)))
    (else
      (goto _label))))

(fn `Handle Slash`
  (params (`Enemy Pet` :type "/Game/Blueprints/PET_BLUEPRINTS/BP_PET_PARENT Object Reference"))
  (locals (EnemyPet :type "/Game/Blueprints/PET_BLUEPRINTS/BP_PET_PARENT Object Reference"))
  (bind _battlelog (`self.battleLog`))
  (bind _battlelog_2 (`self.battleLog`))
  (bind _returnvalue (`AIBlueprintHelperLibrary.GetBlackboard` self))
  (bind _output_get (set `local.EnemyPet` `Enemy Pet`))
  (`BlackboardComponent.SetValueAsInt` _returnvalue "animationstate" 2)
  (`BlackboardComponent.SetValueAsBool` _returnvalue "isAnimating" true)
  (bind _returnvalue_2 (`AIBlueprintHelperLibrary.GetBlackboard` _output_get))
  (`BlackboardComponent.SetValueAsInt` _returnvalue_2 "animationstate" 6)
  (`BlackboardComponent.SetValueAsBool` _returnvalue_2 "isAnimating" true)
  (if (and (> (`KismetMathLibrary.RandomFloat`) 0.05) (>= (`self.mana`) (`self.slashMana`)))
    (set `self.mana` (- (`self.mana`) (`self.slashMana`)))
    (set `/Game/Blueprints/PET_BLUEPRINTS/BP_PET_PARENT.hp` (- (`/Game/Blueprints/PET_BLUEPRINTS/BP_PET_PARENT.hp` (`local.EnemyPet`)) (* (`self.atk`) 2)) (`local.EnemyPet`))
    (if (`BlackboardComponent.GetValueAsBool` (`AIBlueprintHelperLibrary.GetBlackboard` null) "isFriendly")
      (`/Game/Assets/BattleAssets/BP_BattleLog.AddLogEntry` _battlelog "You slashed the enemy!")
      (else
        (`/Game/Assets/BattleAssets/BP_BattleLog.AddLogEntry` _battlelog "Enemy slashed you!")))
    (`GameplayStatics.PlaySound2D` "/Game/Assets/Sounds/SFX/HitHeavy.HitHeavy" 1.0 1.0 0.0 null null)
    (else
      (if (`BlackboardComponent.GetValueAsBool` (`AIBlueprintHelperLibrary.GetBlackboard` null) "isFriendly")
        (`/Game/Assets/BattleAssets/BP_BattleLog.AddLogEntry` _battlelog_2 "Your slash failed!")
        (else
          (`/Game/Assets/BattleAssets/BP_BattleLog.AddLogEntry` _battlelog_2 "Enemy slash failed!")))
      (`GameplayStatics.PlaySound2D` "/Game/Assets/Sounds/SFX/Fail.Fail" 1.0 1.0 0.0 null null))))

(fn `Make Special Move`
  (params (Enemy :type "/Game/Blueprints/PET_BLUEPRINTS/BP_PET_PARENT Object Reference"))
  (bind _level (`self.level`))
  (bind _enemy (`local.Enemy`))
  (if (<= _level 7)
    (`self.Paralyze Enemy` _enemy :!label _label)
    (else
      (if (<= _level 9)
        _
        (elif (> (`KismetMathLibrary.RandomFloat`) 0.5)
          (goto _label)
          (else
            _)))
      (`self.Poison Enemy` _enemy))))

(fn `Paralyze Enemy`
  (params (Enemy :type "/Game/Blueprints/PET_BLUEPRINTS/BP_PET_PARENT Object Reference"))
  (bind _battlelog (`self.battleLog`))
  (bind _battlelog_2 (`self.battleLog`))
  (if (>= (* 0.12 (`self.level`)) (`KismetMathLibrary.RandomFloat`))
    (`GameplayStatics.PlaySound2D` "/Game/Assets/Sounds/SFX/Paralyzed.Paralyzed" 1.0 1.0 0.0 null null)
    (set `/Game/Blueprints/PET_BLUEPRINTS/BP_PET_PARENT.isParalyzed` true (`local.Enemy`))
    (if (`BlackboardComponent.GetValueAsBool` (`AIBlueprintHelperLibrary.GetBlackboard` null) "isFriendly")
      (`/Game/Assets/BattleAssets/BP_BattleLog.AddLogEntry` _battlelog "You paralyzed the enemy!")
      (else
        (`/Game/Assets/BattleAssets/BP_BattleLog.AddLogEntry` _battlelog "You were paralyzed!")))
    (else
      (`GameplayStatics.PlaySound2D` "/Game/Assets/Sounds/SFX/Fail.Fail" 1.0 1.0 0.0 null null)
      (if (`BlackboardComponent.GetValueAsBool` (`AIBlueprintHelperLibrary.GetBlackboard` null) "isFriendly")
        (`/Game/Assets/BattleAssets/BP_BattleLog.AddLogEntry` _battlelog_2 "Your paralyze missed!")
        (else
          (`/Game/Assets/BattleAssets/BP_BattleLog.AddLogEntry` _battlelog_2 "Enemy paralyze missed!"))))))

(fn `Poison Enemy`
  (params (Enemy :type "/Game/Blueprints/PET_BLUEPRINTS/BP_PET_PARENT Object Reference"))
  (bind _battlelog (`self.battleLog`))
  (bind _battlelog_2 (`self.battleLog`))
  (if (>= (* 0.1 (`self.level`)) (`KismetMathLibrary.RandomFloat`))
    (set `/Game/Blueprints/PET_BLUEPRINTS/BP_PET_PARENT.poisonedCounter` (`KismetMathLibrary.Min` 5 (- (`self.level`) 7)) (`local.Enemy`))
    (`GameplayStatics.PlaySound2D` "/Game/Assets/Sounds/SFX/Poison.Poison" 1.0 1.0 0.0 null null)
    (if (`BlackboardComponent.GetValueAsBool` (`AIBlueprintHelperLibrary.GetBlackboard` null) "isFriendly")
      (`/Game/Assets/BattleAssets/BP_BattleLog.AddLogEntry` _battlelog_2 "You poisoned the enemy!")
      (else
        (`/Game/Assets/BattleAssets/BP_BattleLog.AddLogEntry` _battlelog_2 "You were poisoned!")))
    (elif (`BlackboardComponent.GetValueAsBool` (`AIBlueprintHelperLibrary.GetBlackboard` null) "isFriendly")
      (`/Game/Assets/BattleAssets/BP_BattleLog.AddLogEntry` _battlelog "Your poison missed!")
      (else
        (`/Game/Assets/BattleAssets/BP_BattleLog.AddLogEntry` _battlelog "Enemy poison missed!")))))

(fn `Regen Mana`
  (if (not (>= (`self.mana`) (`self.maxMana`)))
    (set `self.mana` (+ (`self.mana`) 1))))

(fn `UserConstructionScript`)