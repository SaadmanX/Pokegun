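; BP_PET_PINK_CHAR is a pink pet character that tracks how far it is from the player.
; On BeginPlay it caches the BP_TopDownChar found in the level and clears its MovingSprite flag.
; Each tick it compares the 2D distance to that player against a fixed threshold, setting MovingSprite true only when farther away.
; The graph only maintains this flag and contains no movement or sprite-switching logic.
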(event `self.ReceiveBeginPlay`
  (bind _returnvalue (`GameplayStatics.GetActorOfClass` "/Game/Blueprints/PLAYER_BLUEPRINTS/BP_TopDownChar.BP_TopDownChar_C"))
  (set `self.Player` _returnvalue)
  (set `self.moving_sprite` false))

(event `self.ReceiveTick`
  (params (DeltaSeconds :type "Float (single-precision)"))
  (`/Engine/EditorBlueprintResources/StandardMacros.CompareFloat` (`KismetMathLibrary.Distance2D` (`KismetMathLibrary.Conv_VectorToVector2D` (`self.K2_GetActorLocation` (`self.Player`))) (`KismetMathLibrary.Conv_VectorToVector2D` (`self.K2_GetActorLocation`))) 110.0
    (:`>`
      (set `self.moving_sprite` true))
    (:`==`
      (set `self.moving_sprite` false :!label _label))
    (:`<`
      (goto _label))))

(fn `UserConstructionScript`)