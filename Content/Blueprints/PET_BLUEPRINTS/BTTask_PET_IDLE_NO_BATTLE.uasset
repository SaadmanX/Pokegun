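; Behavior Tree task that sets a pet AI to its idle, out-of-battle state.
; On execute it reads the player character from the blackboard and writes the pet's distance to the player into the playerdistance key.
; It also sets the animationstate key to idle and finishes successfully at once.
; If the player key does not cast to BP_TopDownChar, the task never calls FinishExecute.
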(event `self.ReceiveExecuteAI`
  (params (OwnerController :type "AIController Object Reference") (ControlledPawn :type "Pawn Object Reference"))
  (bind _returnvalue (`AIBlueprintHelperLibrary.GetBlackboard` OwnerController))
  (bind _asbp_top_down_char (cast `/Game/Blueprints/PLAYER_BLUEPRINTS/BP_TopDownChar` (`BlackboardComponent.GetValueAsObject` _returnvalue "player")))
  (bind _output_get (set `self.playerdistance` (`Actor.GetDistanceTo` _asbp_top_down_char ControlledPawn)))
  (`BlackboardComponent.SetValueAsFloat` _returnvalue "playerdistance" _output_get)
  (`BlackboardComponent.SetValueAsInt` _returnvalue "animationstate" 0)
  (`self.FinishExecute` true))