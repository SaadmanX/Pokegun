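; BP_PET_CONTROLLER is the AI controller for pets, running the BT_PET behavior tree on BeginPlay.
; It finds the BP_TopDownChar player and seeds the blackboard with that reference plus default distance, animation state and pet state values.
; It then casts the controlled pawn to BP_PET_PARENT and copies its IsFriendly flag into the blackboard; Tick and construction script are empty.
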(event `self.ReceiveBeginPlay`
  (bind _returnvalue (`AIBlueprintHelperLibrary.GetBlackboard` null))
  (`self.RunBehaviorTree` "/Game/Blueprints/PET_BLUEPRINTS/BT_PET.BT_PET")
  (bind _returnvalue_2 (`GameplayStatics.GetActorOfClass` "/Game/Blueprints/PLAYER_BLUEPRINTS/BP_TopDownChar.BP_TopDownChar_C"))
  (bind _output_get (set `self.Player` _returnvalue_2))
  (`BlackboardComponent.SetValueAsObject` _returnvalue "player" _output_get)
  (`BlackboardComponent.SetValueAsFloat` _returnvalue "playerdistance" 100000.0)
  (`BlackboardComponent.SetValueAsInt` _returnvalue "animationstate" 100)
  (`BlackboardComponent.SetValueAsBool` _returnvalue "pet_state" false)
  (bind _asbp_pet_parent (cast `/Game/Blueprints/BP_PET_PARENT` (`self.K2_GetPawn`)))
  (`BlackboardComponent.SetValueAsBool` _returnvalue "isFriendly" (`/Game/Blueprints/BP_PET_PARENT.isFriendly` _asbp_pet_parent)))

(event `self.ReceiveTick`
  (params (DeltaSeconds :type "Float (single-precision)")))

(fn `UserConstructionScript`)