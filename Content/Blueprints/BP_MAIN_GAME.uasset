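; BP_MAIN_GAME sets up the player's friendly pets when play begins.
; It finds the BP_TopDownChar player and sets the pet-to-battle name in GI_Game to a hardcoded BP_SPIRIT.
; It then spawns every class in GI_Game's FriendlyPets list near the player, offset by one random scalar added to all axes, height included.
; Each spawned pet's AI blackboard gets isFriendly set to true.
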(event `self.ReceiveBeginPlay`
  (bind _returnvalue (`GameplayStatics.GetActorOfClass` "/Game/Blueprints/PLAYER_BLUEPRINTS/BP_TopDownChar.BP_TopDownChar_C"))
  (set `self.player` _returnvalue)
  (bind _asgi_game (cast `/Game/Blueprints/GI_Game` (`GameplayStatics.GetGameInstance`)))
  (set `/Game/Blueprints/GI_Game.pet_to_battle_with_name` "BP_SPIRIT" _asgi_game)
  (for _array_element (`.pets_3_6CC6D88047201659FDAC67869502CA7C` (break `/Game/Blueprints/FriendlyPets` (`/Game/Blueprints/GI_Game.friendlyPets` _asgi_game)))
    (bind _returnvalue_2 (`|SpawnActorFromClass` _array_element (`KismetMathLibrary.MakeTransform` (+ (`self.K2_GetActorLocation` (`self.player`)) (* (`KismetMathLibrary.RandomFloat`) 1000.0))) "Undefined" "MultiplyWithRoot" null null))
    (`BlackboardComponent.SetValueAsBool` (`AIBlueprintHelperLibrary.GetBlackboard` _returnvalue_2) "isFriendly" true)))

(fn `UserConstructionScript`)