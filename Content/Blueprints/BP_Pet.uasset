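; BP_Pet is a combat pet holding Hp, Mana, Atk and Def, with chance-based actions for a pet-versus-pet battle.
; Attack and Slash damage the enemy pet directly, Slash spending Mana for double damage; Attack refunds the target's Def if its DefSuccess flag is set, then clears it.
; Healing scales current Hp by a random tier, capped at MaxHp.
; Defend only ever clears DefSuccess, never sets it; event graph is empty.
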(event `self.ReceiveBeginPlay`)

(fn `Handle Attack`
  (params (`Enemy Pet` :type "/Game/Blueprints/BP_Pet Object Reference"))
  (locals (EnemyPet :type "/Game/Blueprints/BP_Pet Object Reference"))
  (bind _enemypet (`local.EnemyPet`))
  (set `local.EnemyPet` `Enemy Pet`)
  (if (> (`KismetMathLibrary.RandomFloat`) 0.1)
    (bind _output_get (set `/Game/Blueprints/BP_Pet.hp` (- (`/Game/Blueprints/BP_Pet.hp` (`local.EnemyPet`)) (`self.atk`)) _enemypet))
    (if (`/Game/Blueprints/BP_Pet.defSuccess` (`local.EnemyPet`))
      (set `/Game/Blueprints/BP_Pet.hp` (+ _output_get (`/Game/Blueprints/BP_Pet.def` _enemypet)) (`local.EnemyPet`))
      (set `/Game/Blueprints/BP_Pet.defSuccess` false (`local.EnemyPet`)))
    (else
      (`KismetSystemLibrary.PrintString` "Bad luck, you missed"))))

(fn `Handle Defend`
  (if (> (`KismetMathLibrary.RandomFloat`) 0.4)
    (set `self.defSuccess` false)))

(fn `Handle Healing`
  (bind _maxhp (`self.maxHp`))
  (bind _maxhp_2 (`self.maxHp`))
  (bind _returnvalue (* (`self.hp`) 1.2))
  (bind _returnvalue_2 (* (`self.hp`) 1.1))
  (if (>= (`self.hp`) (`self.maxHp`))
    _
    (elif (>= (`KismetMathLibrary.RandomFloat`) 0.8)
      (if (> _returnvalue _maxhp_2)
        (set `self.hp` _maxhp_2)
        (else
          (set `self.hp` _returnvalue)))
      (elif (> _returnvalue_2 _maxhp)
        (set `self.hp` _maxhp)
        (else
          (set `self.hp` _returnvalue_2))))))

(fn `Handle Slash`
  (params (EnemyPet :type "/Game/Blueprints/BP_Pet Object Reference"))
  (locals (`Enemy Pet` :type "/Game/Blueprints/BP_Pet Object Reference"))
  (set `local.Enemy Pet` EnemyPet)
  (if (and (> (`KismetMathLibrary.RandomFloat`) 0.05) (> (`self.mana`) 0))
    (set `self.mana` (- (`self.mana`) 5))
    (set `/Game/Blueprints/BP_Pet.hp` (- (`/Game/Blueprints/BP_Pet.hp` (`local.Enemy Pet`)) (* (`self.atk`) 2)) (`local.Enemy Pet`))))

(fn `UserConstructionScript`)